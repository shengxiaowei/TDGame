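; Test AI character that hunts BP_pao towers and attacks them until they die.
; MoveAndSearchTarget sphere-traces for towers, picks the nearest within the remembered distance and moves to it via AIMoveTo, calling itself again immediately when none qualifies.
; A looping timer then box-traces along an angled facing until it hits a tower and starts Attack.
; Attack repeats a montage, damaging Tower (last one found by the search, not RefAttackTower) on notifies, and re-searches once it dies.
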(event Custom|Attack
  (bind _tower (Variables|Default|GetTower))
  (bind _is_death_ (Variables|/Game/BP/pao/BP_pao.BP_pao_C|GetIS_Death? _tower))
  (Animation|Montage|PlayMontage (Variables|Character|GetMesh) (Variables|attribute|GetRef_AttackMontage) 1.0 0.0 "Attack1" :!label _label
    (:then
      (Development|PrintString (Utilities|String|ToString(Boolean) _is_death_)))
    (:OnCompleted
      (if _is_death_
        (CallFunction|MoveandSearchTarget)
        (else
          (goto _label))))
    (:OnNotifyBegin
      (bind _returnvalue (Game|Damage|ApplyDamage _tower 1.0 0 self))
      (Development|PrintString (Utilities|String|ToString(Float) _returnvalue)))))

(event Custom|MoveAndSearchTarget
  (bind _returnvalue (Transformation|GetActorLocation))
  (bind (_outhits _returnvalue_2) (Collision|MultiSphereTraceForObjects _returnvalue _returnvalue 2e+03 (Utilities|Array|MakeArray "ObjectTypeQuery8") false 0 "ForDuration"))
  (if _returnvalue_2
    (for _array_element _outhits
      (bind _asbp_pao (Utilities|Casting|CastToBP_pao (.HitActor (Collision|BreakHitResult _array_element))))
      (Variables|Default|SetTower _asbp_pao)
      (Utilities|Array|Add (Variables|Default|Getmubiao) _asbp_pao))
    (if (>= (Utilities|Array|Length (Variables|Default|Getmubiao)) 1)
      (bind _hasenemy (CallFunction|FUCEnemyfromBaseDistance))
      (if _hasenemy
        (AI|AIMoveTo self "0, 0, 0" (Variables|Gaming|GetRef_AttackTower) 5.0 false
          (:then
            (Utilities|FlowControl|Delay 1.0)
            (bind _returnvalue_3 (Utilities|Time|SetTimerbyFunctionName 0 "FUC_AttackSarch" 0.5 true))
            (Variables|Gaming|SetSearchTimer _returnvalue_3)))
        (else
          (CallFunction|MoveandSearchTarget :!label _label)))
      (else
        (goto _label)))))

(event EventBeginPlay
  (CallFunction|MoveandSearchTarget))

(fn ConstructionScript)

(fn FUCAttackSarch
  (bind _returnvalue (Transformation|GetActorRotation))
  (bind _returnvalue_2 (Transformation|GetActorLocation))
  (bind (_roll _pitch _yaw) (Math|Rotator|BreakRotator _returnvalue))
  ;[1 1 1] 搜寻
  (bind (_outhit _returnvalue_3) (Class|KismetSystemLibrary|BoxTraceSingleforObjects _returnvalue_2 (+ (* (Math|Vector|GetForwardVector (Math|Rotator|MakeRotator _roll _pitch (+ _yaw (Variables|attribute|GetAttack%20Angle)))) (Variables|attribute|GetAttackRange)) _returnvalue_2) "50.000000,50.000000,50.000000" "0, 0, 0" (Utilities|Array|MakeArray "ObjectTypeQuery8") false 0 "Persistent" true))
  (if _returnvalue_3
    (bind _asbp_pao (Utilities|Casting|CastToBP_pao (.HitActor (Collision|BreakHitResult _outhit))))
    (Utilities|Time|ClearandInvalidateTimerbyHandle (Variables|Gaming|GetSearchTimer))
    (Variables|Gaming|SetRef_AttackTower _asbp_pao)
    (CallFunction|Attack)))

(fn FUCEnemyfromBaseDistance
  (for _array_element (Variables|Default|Getmubiao)
    (if (<= (Math|Vector|VectorLength (- (Transformation|GetActorLocation) (Transformation|GetActorLocation _array_element))) (LocalVariables|GetenemyDistanceRemember))
      (LocalVariables|SetenemyDistanceRemember (Math|Vector|VectorLength (- (Transformation|GetActorLocation) (Transformation|GetActorLocation _array_element))))
      (Variables|Gaming|SetRef_AttackTower _array_element)))
  (return (Utilities|IsValid (Variables|Gaming|GetRef_AttackTower)) 0))