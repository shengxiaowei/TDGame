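; Enemy character that marches toward the base (BP_jidi) via AIMoveTo and attacks BP_pao towers it meets along the way.
; A looping timer box-traces at an angle off its facing; a hit tower stops movement and starts random attack montage sections, whose notifies apply damage.
; Attacks repeat until the tower is invalid, then the march resumes.
; Incoming damage is reduced by armor with a minimum floor, destroying the enemy at zero health.
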(event Custom|Hit%20Taget
  ;[1 1 1] 击中
  (Game|Damage|ApplyDamage (Variables|Gaming|GetRef_AttackTower) (Variables|attribute|GetBase%20Damage) 0 self))

(event Custom|MoveAndSearchTarget
  (AI|AIMoveTo self "0, 0, 0" (Variables|Gaming|GetRef_jidi) (Variables|Default|GetAcceptance%20Radius) false
    (:then
      (Utilities|FlowControl|Delay 1.0)
      (bind _returnvalue (Utilities|Time|SetTimerbyFunctionName 0 "FUC_AttackSarch" 0.5 true))
      (Variables|Gaming|SetSearchTimer _returnvalue))))

(event Custom|Attack
  (Components|Movement|StopMovementImmediately (Variables|Character|GetCharacterMovement))
  (Variables|Gaming|SetIsAttack? true :!label _label)
  (Animation|Montage|PlayMontage (Variables|Character|GetMesh) (Variables|attribute|GetRef_AttackMontage) 1.0 0.0 (Utilities|String|StringToName (Utilities|String|Append "Attack" (Utilities|String|ToString(Integer) (Math|Random|RandomIntegerinRange 1 (Variables|Default|GetArrackAnimCount)))))
    (:OnCompleted
      (Variables|Gaming|SetIsAttack? false)
      (Utilities|IsValid (Variables|Gaming|GetRef_AttackTower)
        (:Is%20Valid
          (goto _label))
        (:Is%20Not%20Valid
          (CallFunction|MoveandSearchTarget))))
    (:OnNotifyBegin
      (CallFunction|HitTaget))))

(event Custom|EventAnyDamage
  (params (Damage :type Float%20%28single-precision%29) (DamageType :type Damage%20Type%20Object%20Reference) (InstigatedBy :type Controller%20Object%20Reference) (DamageCauser :type Actor%20Object%20Reference))
  (bind _output_get (Variables|attribute|SetEnemy_Health (- (Variables|attribute|GetEnemy_Health) (Math|Float|Clamp(Float) (- Damage (Variables|attribute|GetEnemy_Armor)) 0.1 999.0))))
  (if (<= _output_get 0.0)
    (Variables|Default|SetIS_Death? (<= _output_get 0.0))
    (Actor|DestroyActor)))

(event Game|Damage|EventAnyDamage
  (params (Damage :type Float%20%28single-precision%29) (DamageType :type Damage%20Type%20Object%20Reference) (InstigatedBy :type Controller%20Object%20Reference) (DamageCauser :type Actor%20Object%20Reference))
  ;[1 1 1] 应用伤害
  (bind _output_get (Variables|attribute|SetEnemy_Health (- (Variables|attribute|GetEnemy_Health) (Math|Float|Clamp(Float) (- Damage (Variables|attribute|GetEnemy_Armor)) 0.1 999.0))))
  (if (<= _output_get 0.0)
    (Variables|Default|SetIS_Death? (<= _output_get 0.0))))

(event EventBeginPlay
  (bind _outactors (Actor|GetAllActorsOfClass "/Game/sengling/mesh/jidi/BP_jidi.BP_jidi_C"))
  (Variables|Gaming|SetRef_jidi (Utilities|Array|Get(acopy) _outactors))
  (CallFunction|MoveandSearchTarget))

(fn ConstructionScript)

(fn FUCAttackSarch
  (bind _returnvalue (Transformation|GetActorRotation))
  (bind _returnvalue_2 (Transformation|GetActorLocation))
  (bind (_roll _pitch _yaw) (Math|Rotator|BreakRotator _returnvalue))
  ;[1 1 1] 搜寻
  (bind (_outhit _returnvalue_3) (Class|KismetSystemLibrary|BoxTraceSingleforObjects _returnvalue_2 (+ (* (Math|Vector|GetForwardVector (Math|Rotator|MakeRotator _roll _pitch (+ _yaw (Variables|attribute|GetAttack%20Angle)))) (Variables|attribute|GetAttackRange)) _returnvalue_2) "50.000000,50.000000,50.000000" "0, 0, 0" (Utilities|Array|MakeArray "ObjectTypeQuery8") false 0 "Persistent" true))
  (if _returnvalue_3
    (bind _asbp_pao (Utilities|Casting|CastToBP_pao (.HitActor (Collision|BreakHitResult _outhit))))
    (Utilities|Time|ClearandInvalidateTimerbyHandle (Variables|Gaming|GetSearchTimer))
    (Variables|Gaming|SetRef_AttackTower _asbp_pao)
    (CallFunction|Attack)))

(fn Sousuo1
  (bind _returnvalue (Transformation|GetActorLocation))
  (bind (_outhits _returnvalue_2) (Collision|MultiSphereTraceForObjects _returnvalue _returnvalue 2e+03 (Utilities|Array|MakeArray "ObjectTypeQuery8") false 0 "ForDuration"))
  (if _returnvalue_2
    (for _array_element _outhits
      (bind _asbp_pao (Utilities|Casting|CastToBP_pao (.HitActor (Collision|BreakHitResult _array_element))))
      (Utilities|Array|Add (Variables|Default|GetPao) _asbp_pao))
    (for _array_element_2 (Variables|Default|GetPao)
      (if (<= (Math|Vector|VectorLength (- (Transformation|GetActorLocation _array_element_2) (Transformation|GetActorLocation self))) (Variables|Default|Getjuli))
        (Variables|Default|Setjuli (Math|Vector|VectorLength (- (Transformation|GetActorLocation _array_element_2) (Transformation|GetActorLocation self))))
        (bind _output_get (Variables|Default|Setattckpao _array_element_2))
        (return false _output_get)))))